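; Barbed wire actor for the battlefield that lays wire meshes along an editable spline in its construction script, with no runtime logic.
; It adds a shadowless static mesh every 200 units, lifted by FloorOffset, aimed at the next spline point and X-scaled to the distance between them.
; Unseeded random roll and Y-scale mirroring break up repetition, so the look can change whenever construction reruns.
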(fn `UserConstructionScript`
  (for _index (range (+ (`KismetMathLibrary.FTrunc` (/ (`SplineComponent.GetSplineLength` (`self.MasterSpline`)) 200.0)) 1))
    (bind _returnvalue (`SplineComponent.GetLocationAtDistanceAlongSpline` (`self.MasterSpline`) (`KismetMathLibrary.Conv_IntToDouble` (* _index 200)) "Local"))
    (bind _returnvalue_2 (`SplineComponent.GetLocationAtDistanceAlongSpline` (`self.MasterSpline`) (`KismetMathLibrary.Conv_IntToDouble` (* (+ _index 1) 200)) "Local"))
    (bind (_returnvalue_roll _returnvalue_pitch _returnvalue_yaw) (`KismetMathLibrary.BreakRotator` (`KismetMathLibrary.FindLookAtRotation` _returnvalue _returnvalue_2)))
    (bind _returnvalue_3 (`AddComponent|NODE_AddStaticMeshComponent-0` :`RelativeTransform` (`KismetMathLibrary.MakeTransform` (+ _returnvalue (`KismetMathLibrary.MakeVector` 0.0 0.0 (`self.Floor_Offset`))) (`KismetMathLibrary.MakeRotator` (+ _returnvalue_roll (`KismetMathLibrary.RandomInteger` 180)) _returnvalue_pitch _returnvalue_yaw) (`KismetMathLibrary.MakeVector` (/ (`KismetMathLibrary.Vector_Distance` _returnvalue _returnvalue_2) 200.0) (`KismetMathLibrary.Conv_IntToDouble` (- 1 (* (`KismetMathLibrary.Conv_BoolToInt` (`KismetMathLibrary.RandomBool`)) 2))) 1.0))))
    (`StaticMeshComponent.SetStaticMesh` _returnvalue_3 "/Game/Battlefield/StaticMeshes/Props/SM_BarbedWire_01.SM_BarbedWire_01")
    (`PrimitiveComponent.SetCastShadow` _returnvalue_3 false)))