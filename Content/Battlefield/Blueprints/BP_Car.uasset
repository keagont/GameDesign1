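; BP_Car is a Battlefield prop actor that randomizes a car's appearance in its Construction Script, with no active gameplay logic.
; A weighted roll adds four wheels at WheelPlacement transforms, each with its own weighted chance of a tire.
; The body is an instanced static mesh component, set lower when wheelless and randomly given one of two car meshes.
; The rolls are unseeded, so the look changes whenever construction reruns.
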(fn `UserConstructionScript`
  (bind _car (`self.Car`))
  (if (`KismetMathLibrary.RandomBoolWithWeight` (`self.HasWheels? WeightBias`))
    (for _index (range 4)
      (bind _output (`|GetArrayItem` (`self.WheelPlacement`) _index))
      (bind _returnvalue (`AddComponent|NODE_AddStaticMeshComponent-0` :`RelativeTransform` _output))
      (`StaticMeshComponent.SetStaticMesh` _returnvalue "/Game/Battlefield/StaticMeshes/Rubble/SM_Wheel_01.SM_Wheel_01")
      (if (`KismetMathLibrary.RandomBoolWithWeight` (`self.HasTires? WeightBias`))
        (bind _returnvalue_2 (`AddComponent|NODE_AddStaticMeshComponent-1` :`RelativeTransform` _output))
        (`StaticMeshComponent.SetStaticMesh` _returnvalue_2 "/Game/Battlefield/StaticMeshes/Rubble/SM_Tire_01.SM_Tire_01")))
    (bind _returnvalue_3 (`AddComponent|NODE_AddInstancedStaticMeshComponent-1` :`RelativeTransform` (`KismetMathLibrary.MakeTransform` (0.0 0.0 30.0))))
    (set `self.Car` _returnvalue_3)
    (else
      (bind _returnvalue_4 (`AddComponent|NODE_AddInstancedStaticMeshComponent-0` :`RelativeTransform` (`KismetMathLibrary.MakeTransform` (0.0 0.0 10.0))))
      (set `self.Car` _returnvalue_4)))
  (if (`KismetMathLibrary.RandomBool`)
    (`StaticMeshComponent.SetStaticMesh` _car "/Game/Battlefield/StaticMeshes/Cars/SM_Car_A_01.SM_Car_A_01")
    (else
      (`StaticMeshComponent.SetStaticMesh` _car "/Game/Battlefield/StaticMeshes/Cars/SM_Car_B_01.SM_Car_B_01"))))