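; BP_FenceBlocks is a battlefield prop that builds a randomized tarped fence segment with a concrete block.
; The construction script adds both mesh components, randomly mirroring each on Y and placing the block on either side of the fence.
; Cascaded weighted rolls pick among four fence meshes about equally, while the block strongly favors one of two meshes.
; Randomness is unseeded and the event graph has no active logic.
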(fn `UserConstructionScript`
  (bind _returnvalue (`KismetMathLibrary.Conv_BoolToInt` (`KismetMathLibrary.RandomBoolWithWeight` 0.5)))
  (bind _returnvalue_2 (`AddComponent|NODE_AddStaticMeshComponent-0` :`RelativeTransform` (`KismetMathLibrary.MakeTransform` (`KismetMathLibrary.MakeVector` 20.0 (`KismetMathLibrary.Conv_IntToDouble` (- 30 (* 70 _returnvalue)))) (struct) (`KismetMathLibrary.MakeVector` 1.0 (`KismetMathLibrary.Conv_IntToDouble` (- 1 (* _returnvalue 2))) 1.0))))
  (if (`KismetMathLibrary.RandomBoolWithWeight` 0.8)
    (`StaticMeshComponent.SetStaticMesh` _returnvalue_2 "/Game/Battlefield/StaticMeshes/Concrete_Barriers/SM_ConcreteBlock_03.SM_ConcreteBlock_03")
    (else
      (`StaticMeshComponent.SetStaticMesh` _returnvalue_2 "/Game/Battlefield/StaticMeshes/Concrete_Barriers/SM_ConcreteBlock_02.SM_ConcreteBlock_02")))
  (bind _returnvalue_3 (`AddComponent|NODE_AddStaticMeshComponent-1` :`RelativeTransform` (`KismetMathLibrary.MakeTransform` (0.0 0.0 0.0) (struct) (`KismetMathLibrary.MakeVector` 1.0 (`KismetMathLibrary.Conv_IntToDouble` (- 1 (* (`KismetMathLibrary.Conv_BoolToInt` (`KismetMathLibrary.RandomBoolWithWeight` 0.5)) 2))) 1.0))))
  (if (`KismetMathLibrary.RandomBoolWithWeight` 0.25)
    (`StaticMeshComponent.SetStaticMesh` _returnvalue_3 "/Game/Battlefield/StaticMeshes/Concrete_Barriers/SM_TarpedFence_01.SM_TarpedFence_01")
    (elif (`KismetMathLibrary.RandomBoolWithWeight` 0.33)
      (`StaticMeshComponent.SetStaticMesh` _returnvalue_3 "/Game/Battlefield/StaticMeshes/Concrete_Barriers/SM_TarpedFence_02.SM_TarpedFence_02")
      (elif (`KismetMathLibrary.RandomBoolWithWeight` 0.5)
        (`StaticMeshComponent.SetStaticMesh` _returnvalue_3 "/Game/Battlefield/StaticMeshes/Concrete_Barriers/SM_TarpedFence_01a.SM_TarpedFence_01a")
        (else
          (`StaticMeshComponent.SetStaticMesh` _returnvalue_3 "/Game/Battlefield/StaticMeshes/Concrete_Barriers/SM_TarpedFence_02a.SM_TarpedFence_02a"))))))