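; Spline-driven fence actor for dressing battlefield levels, built entirely in the Construction Script.
; It sets all spline points to linear or curved, then spawns fixed-length fence meshes along the spline, each aimed at the next with near-flat pitch.
; Weighted random picks vary tarped and plain fence meshes, with random Y mirroring.
; An optional second pass adds random concrete block meshes that follow slopes more steeply.
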(fn `UserConstructionScript`
  (bind _masterspline (`self.MasterSpline`))
  (bind _masterspline_2 (`self.MasterSpline`))
  (bind _masterspline_3 (`self.MasterSpline`))
  (bind _returnvalue (`KismetMathLibrary.FTrunc` (/ (`SplineComponent.GetSplineLength` _masterspline) 245.0)))
  (if (`self.Linear`)
    (for _index (range (+ (`SplineComponent.GetNumberOfSplinePoints` _masterspline) 1))
      (`SplineComponent.SetSplinePointType` _masterspline _index "Linear" true))
    (else
      (for _index_2 (range (+ (`SplineComponent.GetNumberOfSplinePoints` _masterspline) 1))
        (`SplineComponent.SetSplinePointType` _masterspline _index_2 "Curve" true))))
  (for _index_3 (range (+ _returnvalue 1))
    (bind _returnvalue_2 (`KismetMathLibrary.Conv_IntToDouble` (* _index_3 245)))
    (bind _returnvalue_3 (`SplineComponent.GetLocationAtDistanceAlongSpline` _masterspline_3 _returnvalue_2 "Local"))
    (bind (_returnvalue_roll _returnvalue_pitch _returnvalue_yaw) (`KismetMathLibrary.BreakRotator` (`KismetMathLibrary.FindLookAtRotation` _returnvalue_3 (`SplineComponent.GetLocationAtDistanceAlongSpline` _masterspline_3 (+ _returnvalue_2 245.0) "Local"))))
    (bind _returnvalue_4 (`AddComponent|NODE_AddStaticMeshComponent-3` :`RelativeTransform` (`KismetMathLibrary.MakeTransform` _returnvalue_3 (`KismetMathLibrary.MakeRotator` _returnvalue_roll (`KismetMathLibrary.ClampAngle` _returnvalue_pitch -1.0 1.0) _returnvalue_yaw) (`KismetMathLibrary.MakeVector` 1.0 (`KismetMathLibrary.Conv_IntToDouble` (- 1 (* (`KismetMathLibrary.Conv_BoolToInt` (`KismetMathLibrary.RandomBool`)) 2))) 1.0))))
    (if (`KismetMathLibrary.RandomBoolWithWeight` 0.25)
      (`StaticMeshComponent.SetStaticMesh` _returnvalue_4 "/Game/Battlefield/StaticMeshes/Concrete_Barriers/SM_TarpedFence_01.SM_TarpedFence_01")
      (elif (`KismetMathLibrary.RandomBoolWithWeight` 0.33)
        (`StaticMeshComponent.SetStaticMesh` _returnvalue_4 "/Game/Battlefield/StaticMeshes/Concrete_Barriers/SM_TarpedFence_02.SM_TarpedFence_02")
        (elif (`KismetMathLibrary.RandomBoolWithWeight` 0.5)
          (`StaticMeshComponent.SetStaticMesh` _returnvalue_4 "/Game/Battlefield/StaticMeshes/Concrete_Barriers/SM_TarpedFence_01a.SM_TarpedFence_01a")
          (elif (`KismetMathLibrary.RandomBoolWithWeight` 0.7)
            (`StaticMeshComponent.SetStaticMesh` _returnvalue_4 "/Game/Battlefield/StaticMeshes/Concrete_Barriers/SM_TarpedFence_02a.SM_TarpedFence_02a")
            (else
              (`StaticMeshComponent.SetStaticMesh` _returnvalue_4 "/Game/Battlefield/StaticMeshes/Concrete_Barriers/SM_Fence_01.SM_Fence_01")))))))
  (if (`self.Add ConcreteBlocks`)
    (for _index_4 (range (+ _returnvalue 1))
      (bind _returnvalue_5 (`KismetMathLibrary.Conv_IntToDouble` (* _index_4 245)))
      (bind _returnvalue_6 (`SplineComponent.GetLocationAtDistanceAlongSpline` _masterspline_2 _returnvalue_5 "Local"))
      (bind (_returnvalue_roll_2 _returnvalue_pitch_2 _returnvalue_yaw_2) (`KismetMathLibrary.BreakRotator` (`KismetMathLibrary.FindLookAtRotation` _returnvalue_6 (`SplineComponent.GetLocationAtDistanceAlongSpline` _masterspline_2 (+ _returnvalue_5 245.0) "Local"))))
      (bind _returnvalue_7 (`AddComponent|NODE_AddStaticMeshComponent-5` :`RelativeTransform` (`KismetMathLibrary.MakeTransform` _returnvalue_6 (`KismetMathLibrary.MakeRotator` _returnvalue_roll_2 (`KismetMathLibrary.ClampAngle` _returnvalue_pitch_2 -30.0 30.0) _returnvalue_yaw_2) (1.0 1.0 1.0))))
      (if (`KismetMathLibrary.RandomBoolWithWeight` 0.5)
        (`StaticMeshComponent.SetStaticMesh` _returnvalue_7 "/Game/Battlefield/StaticMeshes/Concrete_Barriers/SM_ConcreteBlock_03.SM_ConcreteBlock_03")
        (elif (`KismetMathLibrary.RandomBoolWithWeight` 0.5)
          (`StaticMeshComponent.SetStaticMesh` _returnvalue_7 "/Game/Battlefield/StaticMeshes/Concrete_Barriers/SM_ConcreteBlock_03Inverted.SM_ConcreteBlock_03Inverted")
          (elif (`KismetMathLibrary.RandomBoolWithWeight` 0.7)
            (`StaticMeshComponent.SetStaticMesh` _returnvalue_7 "/Game/Battlefield/StaticMeshes/Concrete_Barriers/SM_ConcreteBlock_02.SM_ConcreteBlock_02")
            (else
              (`StaticMeshComponent.SetStaticMesh` _returnvalue_7 "/Game/Battlefield/StaticMeshes/Concrete_Barriers/SM_ConcreteBlock_02Inverted.SM_ConcreteBlock_02Inverted"))))))))