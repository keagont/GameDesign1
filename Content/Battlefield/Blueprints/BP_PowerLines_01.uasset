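; BP_PowerLines_01 is a spline-driven placement actor that builds a line of telephone poles and wires in the level.
; The Construction Script puts a pole with random yaw at each MasterSpline point.
; Between neighboring points it adds a wire mesh at a fixed height, aimed at the next pole and scaled along X to span the gap.
; A downward line trace is left unconnected, and no gameplay logic runs.
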(fn `UserConstructionScript`
  (bind _masterspline (`self.MasterSpline`))
  (bind _masterspline_2 (`self.MasterSpline`))
  (bind _returnvalue (- (`SplineComponent.GetNumberOfSplinePoints` _masterspline) 1))
  (`SplineComponent.SetSplinePointType` (`self.MasterSpline`) 0 "Linear" true)
  (for _index (range (+ _returnvalue 1))
    (bind _returnvalue_2 (`AddComponent|NODE_AddStaticMeshComponent-0` :`RelativeTransform` (`KismetMathLibrary.MakeTransform` (`SplineComponent.GetLocationAtSplinePoint` _masterspline _index "Local") (`KismetMathLibrary.MakeRotator` 0.0 0.0 (`KismetMathLibrary.RandomFloatInRange` -45.0 45.0)))))
    (`StaticMeshComponent.SetStaticMesh` _returnvalue_2 "/Game/Battlefield/StaticMeshes/Props/SM_TelephonePole.SM_TelephonePole"))
  (for _index_2 (range _returnvalue)
    (bind _returnvalue_3 (+ (`SplineComponent.GetLocationAtSplinePoint` _masterspline_2 _index_2 "Local") (0.0 0.0 790.0)))
    (bind _returnvalue_4 (+ (`SplineComponent.GetLocationAtSplinePoint` _masterspline_2 (+ _index_2 1) "Local") (0.0 0.0 790.0)))
    (bind _returnvalue_5 (`AddComponent|NODE_AddStaticMeshComponent-1` :`RelativeTransform` (`KismetMathLibrary.MakeTransform` _returnvalue_3 (`KismetMathLibrary.FindLookAtRotation` _returnvalue_3 _returnvalue_4) (`KismetMathLibrary.MakeVector` (/ (`KismetMathLibrary.Vector_Distance` _returnvalue_3 _returnvalue_4) 1200.0) 1.0 1.0))))
    (`StaticMeshComponent.SetStaticMesh` _returnvalue_5 "/Game/Battlefield/StaticMeshes/Props/SM_Wire_01.SM_Wire_01")))