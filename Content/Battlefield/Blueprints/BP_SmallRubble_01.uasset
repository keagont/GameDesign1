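; Construction-script scatter actor that fills a strip along a spline with small concrete rubble for the Battlefield environment.
; Unless disabled, it fits a Box to the spline's length and LengthY, then adds static mesh components between the first two points' X values.
; Each gets a random yaw, scale and one of three meshes, with weighted Y-offset bias.
; Randomness is unseeded, so layouts change on reconstruction; event graph is empty.
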(fn `UserConstructionScript`
  (bind _returnvalue (`KismetMathLibrary.RandomInteger` 2))
  (bind _spline (`self.Spline`))
  (bind _spline_2 (`self.Spline`))
  (bind _returnvalue_x (`KismetMathLibrary.BreakVector` (`SplineComponent.GetLocationAtSplinePoint` _spline 1 "Local")))
  (bind _returnvalue_x_2 (`KismetMathLibrary.BreakVector` (`SplineComponent.GetLocationAtSplinePoint` _spline 0 "Local")))
  (bind _returnvalue_2 (`SplineComponent.GetSplineLength` _spline_2))
  (bind _returnvalue_3 (/ (`self.Length_Y`) 2.0))
  (bind (_returnvalue_x_3 _returnvalue_y _returnvalue_z) (`KismetMathLibrary.BreakVector` (`SplineComponent.GetLocationAtDistanceAlongSpline` _spline_2 (/ _returnvalue_2 2.0) "Local")))
  (if (not (`self.Disable`))
    (`SceneComponent.K2_SetRelativeTransform` (`self.Box`) (`KismetMathLibrary.MakeTransform` (`KismetMathLibrary.MakeVector` _returnvalue_x_3 _returnvalue_y _returnvalue_z) (struct) (`KismetMathLibrary.MakeVector` (/ _returnvalue_2 50.0) (/ (`self.Length_Y`) 50.0) 1.0)) false false)
    (for _ (range (+ (`self.Number of Instances`) 1))
      (bind _returnvalue_4 (`AddComponent|NODE_AddStaticMeshComponent-0` :`RelativeTransform` (`KismetMathLibrary.MakeTransform` (`KismetMathLibrary.MakeVector` (`KismetMathLibrary.RandomFloatInRange` _returnvalue_x_2 _returnvalue_x) (`KismetMathLibrary.RandomFloatInRange` (+ (- 0.0 _returnvalue_3) (* (`KismetMathLibrary.Conv_BoolToInt` (`KismetMathLibrary.RandomBoolWithWeight` (`self.Offset Bias`))) (`self.Offset Weight_Y`))) _returnvalue_3)) (`KismetMathLibrary.MakeRotator` 0.0 0.0 (`KismetMathLibrary.RandomFloatInRange` -90.0 90.0)) (* (`self.Scale`) (`KismetMathLibrary.Conv_DoubleToVector` (`KismetMathLibrary.RandomFloatInRange` 0.7 1.5))))))
      (if (== _returnvalue 0)
        (`StaticMeshComponent.SetStaticMesh` _returnvalue_4 (`self.Mesh_01`))
        (elif (== _returnvalue 1)
          (`StaticMeshComponent.SetStaticMesh` _returnvalue_4 (`self.Mesh_02`))
          (else
            (`StaticMeshComponent.SetStaticMesh` _returnvalue_4 (`self.Mesh_03`)))))
      (`PrimitiveComponent.SetMaterial` _returnvalue_4 0 "/Game/Battlefield/Materials/Layers/Instances/MI_Concrete_13.MI_Concrete_13"))))