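; Spline-driven wooden fence that builds itself from static mesh segments in the construction script.
; A Linear flag sets every spline point to linear or curve, then fixed-length panels are placed along MasterSpline, each aimed at the next point with pitch clamped nearly level.
; Panels randomly use one of two meshes, and full panels are randomly mirrored on Y.
; A leftover gap of at least half a panel gets an X-scaled end piece.
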(fn `UserConstructionScript`
  (bind _masterspline (`self.MasterSpline`))
  (bind _masterspline_2 (`self.MasterSpline`))
  (bind _masterspline_3 (`self.MasterSpline`))
  (bind _returnvalue (`SplineComponent.GetLocationAtDistanceAlongSpline` _masterspline_3 (`SplineComponent.GetSplineLength` _masterspline_3) "Local"))
  (bind _returnvalue_2 (`KismetMathLibrary.FTrunc` (/ (`SplineComponent.GetSplineLength` _masterspline_2) 413.0)))
  (bind _returnvalue_3 (`SplineComponent.GetLocationAtDistanceAlongSpline` _masterspline_3 (`KismetMathLibrary.Conv_IntToDouble` (* _returnvalue_2 413)) "Local"))
  (bind (_returnvalue_roll _returnvalue_pitch _returnvalue_yaw) (`KismetMathLibrary.BreakRotator` (`KismetMathLibrary.FindLookAtRotation` _returnvalue_3 _returnvalue)))
  (bind _returnvalue_4 (/ (`KismetMathLibrary.VSize` (- _returnvalue_3 _returnvalue)) 413.0))
  (if (`self.Linear`)
    (for _index (range (+ (`SplineComponent.GetNumberOfSplinePoints` _masterspline_2) 1))
      (`SplineComponent.SetSplinePointType` _masterspline_2 _index "Linear" true))
    (else
      (for _index_2 (range (+ (`SplineComponent.GetNumberOfSplinePoints` _masterspline_2) 1))
        (`SplineComponent.SetSplinePointType` _masterspline_2 _index_2 "Curve" true))))
  (for _index_3 (range _returnvalue_2)
    (bind _returnvalue_5 (`KismetMathLibrary.Conv_IntToDouble` (* _index_3 413)))
    (bind _returnvalue_6 (`SplineComponent.GetLocationAtDistanceAlongSpline` _masterspline _returnvalue_5 "Local"))
    (bind (_returnvalue_roll_2 _returnvalue_pitch_2 _returnvalue_yaw_2) (`KismetMathLibrary.BreakRotator` (`KismetMathLibrary.FindLookAtRotation` _returnvalue_6 (`SplineComponent.GetLocationAtDistanceAlongSpline` _masterspline (+ _returnvalue_5 413.0) "Local"))))
    (bind _returnvalue_7 (`AddComponent|NODE_AddStaticMeshComponent-3` :`RelativeTransform` (`KismetMathLibrary.MakeTransform` _returnvalue_6 (`KismetMathLibrary.MakeRotator` _returnvalue_roll_2 (`KismetMathLibrary.ClampAngle` _returnvalue_pitch_2 -1.0 1.0) _returnvalue_yaw_2) (`KismetMathLibrary.MakeVector` 1.0 (`KismetMathLibrary.Conv_IntToDouble` (- 1 (* (`KismetMathLibrary.Conv_BoolToInt` (`KismetMathLibrary.RandomBool`)) 2))) 1.0))))
    (if (`KismetMathLibrary.RandomBoolWithWeight` 0.5)
      (`StaticMeshComponent.SetStaticMesh` _returnvalue_7 "/Game/Battlefield/StaticMeshes/Modular/Shacks/SM_Wooden_Femce_01.SM_Wooden_Femce_01")
      (else
        (`StaticMeshComponent.SetStaticMesh` _returnvalue_7 "/Game/Battlefield/StaticMeshes/Modular/Shacks/SM_Wooden_Femce_02.SM_Wooden_Femce_02"))))
  (if (not (< _returnvalue_4 0.5))
    (bind _returnvalue_8 (`AddComponent|NODE_AddStaticMeshComponent-6` :`RelativeTransform` (`KismetMathLibrary.MakeTransform` _returnvalue_3 (`KismetMathLibrary.MakeRotator` _returnvalue_roll (`KismetMathLibrary.ClampAngle` _returnvalue_pitch -1.0 1.0) _returnvalue_yaw) (`KismetMathLibrary.MakeVector` _returnvalue_4 1.0 1.0))))
    (if (`KismetMathLibrary.RandomBoolWithWeight` 0.5)
      (`StaticMeshComponent.SetStaticMesh` _returnvalue_8 "/Game/Battlefield/StaticMeshes/Modular/Shacks/SM_Wooden_Femce_01.SM_Wooden_Femce_01")
      (else
        (`StaticMeshComponent.SetStaticMesh` _returnvalue_8 "/Game/Battlefield/StaticMeshes/Modular/Shacks/SM_Wooden_Femce_02.SM_Wooden_Femce_02")))))