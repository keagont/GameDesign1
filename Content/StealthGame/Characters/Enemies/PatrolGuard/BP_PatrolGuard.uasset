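; Patrol guard enemy for a stealth game that patrols, investigates noises, searches, and chases the player.
; Tick selects chase, search, or random/waypoint patrol from PawnSensing-driven flags, with CanMove gating AIMoveTo calls and chase requiring a sight-time threshold.
; Retriggerable delays step lost sight down to searching, then patrol.
; Attack montage notifies sphere-trace from the hand to reload the player's checkpoint; a dialogue sphere feeds timed HUD captions once.
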(event `self.DialogueSphere.OnComponentBeginOverlap`
  (params (OverlappedComponent :type "PrimitiveComponent Object Reference") (OtherActor :type "Actor Object Reference") (OtherComp :type "PrimitiveComponent Object Reference") (OtherBodyIndex :type Integer) (bFromSweep :type Boolean) (SweepResult :type "HitResult Structure (by ref)"))
  (bind _talkdialogue (`self.TalkDialogue`))
  (bind _asbp_third_person_character_custom (cast `/Game/StealthGame/Core/Characters/PlayerCharacter/BP_ThirdPersonCharacterCustom` OtherActor))
  (if (> (`KismetArrayLibrary.Array_Length` _talkdialogue) 0)
    (`/Engine/EditorBlueprintResources/StandardMacros.DoOnce` false
      (:`Completed`
        (bind _array_element (`/Game/StealthGame/Core/BML_MacroLibrary.ForEachWithDelay` _talkdialogue 5.0)
          (:`Loop Body`
            (`/Game/StealthGame/Core/Characters/PlayerCharacter/Widgets/W_HUD.AddCaption` (`/Game/StealthGame/Core/Characters/PlayerCharacter/BP_ThirdPersonCharacterCustom.HUD` _asbp_third_person_character_custom) (`self.NameColor`) (`self.Name`) _array_element)))))))

(event `self.PawnSensing.OnSeePawn`
  (params (Pawn :type "Pawn Object Reference"))
  (`|ExecutionSequence`
    (:`then_0`
      (cast `/Game/StealthGame/Core/Characters/PlayerCharacter/BP_ThirdPersonCharacterCustom` Pawn)
      (`KismetSystemLibrary.PrintString` "Get a load of this guy!")
      (set `self.bPlayerVisible` true))
    (:`then_1`
      (`KismetSystemLibrary.RetriggerableDelay` 1.0)
      (`KismetSystemLibrary.PrintString` "Heh... Musta been the wind...")
      (set `self.bPlayerVisible` false)
      (set `self.bPlayerNear` true)
      (`KismetSystemLibrary.PrintString` "But maybe I should search first...")
      (`KismetSystemLibrary.RetriggerableDelay` 10.0)
      (`KismetSystemLibrary.PrintString` "Really was the wind...")
      (set `self.bPlayerNear` false))))

(event `self.ReceiveTick`
  (params (DeltaSeconds :type "Float (single-precision)"))
  (bind _returnvalue (and (`self.bPlayerVisible`) (>= (`self.PlayerInSightTime`) (`self.PlayerMaxSightTime`))))
  (`|ExecutionSequence`
    (:`then_0`
      (if (`self.bCanMove`)
        (if _returnvalue
          (`self.ChasePlayer`)
          (elif (`self.bPlayerNear`)
            (`self.SearchRandomly`)
            (elif (`self.bPatrolRandom`)
              (`self.PatrolRandom`)
              (else
                (`self.MoveToNextPatrolPoint`)))))
        (elif _returnvalue
          (`self.ChasePlayer`))))
    (:`then_1`
      (if true
        _))))

(event `PatrolRandom`
  (`self.UpdateWalkSpeed` 200.0)
  (set `self.bCanMove` false)
  (`|AIMoveTo` self (`NavigationSystemV1.K2_GetRandomReachablePointInRadius` (`self.K2_GetActorLocation`) 2000.0 null null) null
    (:`OnSuccess`
      _)
    (:`OnFail`
      _))
  (`KismetSystemLibrary.Delay` 3.0)
  (set `self.bCanMove` true))

(event `ChasePlayer`
  (`self.UpdateWalkSpeed` 550.0)
  (set `self.bCanMove` false)
  (`|AIMoveTo` self (0.0 0.0 0.0) (`GameplayStatics.GetPlayerCharacter` 0) 50.0
    (:`OnSuccess`
      (`self.Attack`))
    (:`OnFail`
      _))
  (`KismetSystemLibrary.Delay` 3.0)
  (set `self.bCanMove` true))

(event `MoveToNextPatrolPoint`
  (`self.UpdateWalkSpeed` 300.0)
  (set `self.bCanMove` false)
  (`|AIMoveTo` self (0.0 0.0 0.0) (`|GetArrayItem` (`self.PatrolTargetPoints`) (`self.PatrolPointIndex`))
    (:`OnSuccess`
      (`KismetSystemLibrary.Delay` 3.0)
      (set `self.bCanMove` true)
      (`self.SetNextPatrolPointIndex`))
    (:`OnFail`
      (`KismetSystemLibrary.Delay` 3.0)
      (set `self.bCanMove` true))))

(event `SetNextPatrolPointIndex`
  (set `self.PatrolPointIndex` (mod (+ (`self.PatrolPointIndex`) 1) (`KismetArrayLibrary.Array_Length` (`self.PatrolTargetPoints`)))))

(event `SearchRandomly`
  (bind (_returnvalue_roll _returnvalue_pitch _returnvalue_yaw) (`KismetMathLibrary.BreakRotator` (`self.K2_GetActorRotation`)))
  (`self.UpdateWalkSpeed` 200.0)
  (set `self.bCanMove` false)
  (`self.K2_SetActorRotation` (`KismetMathLibrary.MakeRotator` _returnvalue_roll _returnvalue_pitch (+ _returnvalue_yaw (`KismetMathLibrary.RandomFloatInRange` -90.0 90.0))))
  (`KismetSystemLibrary.Delay` 1.0)
  (`|AIMoveTo` self (`NavigationSystemV1.K2_GetRandomReachablePointInRadius` (`self.K2_GetActorLocation`) 300.0 null null) null
    (:`OnSuccess`
      _)
    (:`OnFail`
      _))
  (`KismetSystemLibrary.Delay` 1.5)
  (set `self.bCanMove` true))

(event `self.PawnSensing.OnHearNoise`
  (params (Instigator :type "Pawn Object Reference") (Location :type "Vector Structure (by ref)") (Volume :type "Float (single-precision)"))
  (`KismetSystemLibrary.PrintString` "Weird Noise")
  (set `self.bDistracted` true)
  (`self.UpdateWalkSpeed` 200.0)
  (set `self.bCanMove` false)
  (`|AIMoveTo` self Location Instigator
    (:`OnSuccess`
      _)
    (:`OnFail`
      _))
  (`KismetSystemLibrary.Delay` 6.0) ; Distraction Time
  (set `self.bCanMove` true)
  (set `self.bDistracted` false))

(event `Attack`
  (bind _returnvalue (`SceneComponent.GetSocketLocation` (`self.Mesh`) "hand_r"))
  ;[0.15 0.1407 0.04319 0.5] Bonk
  (`/Engine/EditorBlueprintResources/StandardMacros.DoOnce` false :!label _label ; Only Reset Attack on miss.
    (:`Completed`
      (bind _notifyname (`|PlayMontage` (`self.Mesh`) "/Game/StealthGame/Characters/Enemies/AM_Attack_01.AM_Attack_01") ; Play the AM_Attack_01
        (:`OnCompleted`
          (if (`self.bHostile`)
            (`self.ResetAttack`) ; Resets the Do Once node.
          ))
        (:`OnNotifyBegin`
          (switch `name` _notifyname ; Pick the proper attack type(standard when there is more than one type of attack)
            (:`AttackDamage`
              (`KismetSystemLibrary.PrintString` "I'm attacking!")
              (bind (_outhits _returnvalue_2) (`KismetSystemLibrary.SphereTraceMultiForObjects` _returnvalue (+ _returnvalue (* (`self.GetActorForwardVector`) (`self.MeleeTraceDistance`))) (`self.MeleeTraceRadius`) (`|MakeArray` "ObjectTypeQuery3" :!type "EObjectTypeQuery Enum"))) ; Trace forward from hand socket.
              (if _returnvalue_2
                (for _array_element _outhits
                  (bind _asbp_third_person_character_custom (cast `/Game/StealthGame/Core/Characters/PlayerCharacter/BP_ThirdPersonCharacterCustom` (`.HitActor` (`GameplayStatics.BreakHitResult` _array_element))))
                  (`/Game/StealthGame/Core/Characters/PlayerCharacter/BP_ThirdPersonCharacterCustom.LoadCheckpoint` _asbp_third_person_character_custom)
                  (set `self.bHostile` false))))))))))

(event `ResetAttack`
  ;[0.15 0.1407 0.04319 0.5] Bonk
  (goto _label :!via `Reset`))

(fn `UpdateWalkSpeed`
  (params (newWalkSpeed :type "Float (double-precision)"))
  (set `CharacterMovementComponent.MaxWalkSpeed` newWalkSpeed (`self.CharacterMovement`)))

(fn `UserConstructionScript`)