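; BP_BallSpawner is an interactable actor that sweeps back and forth along the world X axis and can drop balls.
; Tick sets its X position from a sine of game time around a fixed world-space center, keeping Y and Z unchanged.
; DropBall spawns a BP_Ball just below the spawner's current location.
; Nothing in this Blueprint calls DropBall itself.
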(event `self.ReceiveTick`
  (params (DeltaSeconds :type "Float (single-precision)"))
  (bind (_returnvalue_x _returnvalue_y _returnvalue_z) (`KismetMathLibrary.BreakVector` (`self.K2_GetActorLocation`)))
  (`self.K2_SetActorLocation` (`KismetMathLibrary.MakeVector` (+ (* (`KismetMathLibrary.Sin` (* (`KismetSystemLibrary.GetGameTimeInSeconds`) 1.0)) 1200.0) 1500.0) _returnvalue_y _returnvalue_z)))

(event `self.ReceiveBeginPlay`)

(fn `Drop Ball`
  (bind (_returnvalue_x _returnvalue_y _returnvalue_z) (`KismetMathLibrary.BreakVector` (`self.K2_GetActorLocation`)))
  (`|SpawnActorFromClass` "/Game/StealthGame/Core/Interactables/BP_Ball.BP_Ball_C" (`KismetMathLibrary.MakeTransform` (`KismetMathLibrary.MakeVector` _returnvalue_x _returnvalue_y (- _returnvalue_z 50.0))) "Undefined" "MultiplyWithRoot" null null))

(fn `UserConstructionScript`)