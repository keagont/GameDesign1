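; BP_GambleBox is an interactable that fronts a ball-drop gambling setup in the stealth game.
; On BeginPlay it discovers its BP_BallSpawner and BP_GambleCam by casting the actors overlapping it, so the link depends on placement.
; DropBall forwards to that spawner, while SwapCam switches the first player's view between the gamble camera, with a blend, and the third-person character.
; Debug prints report overlapped actors and camera swaps.
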(event `self.ReceiveBeginPlay`
  (for _array_element (`self.GetOverlappingActors` null)
    (`KismetSystemLibrary.PrintString` (`KismetSystemLibrary.GetDisplayName` _array_element) true true (struct :`R` 1.0 :`G` 0.002965 :`B` 0.009651 :`A` 1.0) 5.0)
    (bind _asbp_ball_spawner (cast `/Game/StealthGame/Core/Interactables/BP_BallSpawner` _array_element)
      (:`then`
        (set `self.BallSpawner` _asbp_ball_spawner))
      (:`CastFailed`
        (bind _asbp_gamble_cam (cast `/Game/StealthGame/Core/Interactables/BP_GambleCam` _array_element))
        (set `self.GambleCam` _asbp_gamble_cam)))))

(event `/Game/StealthGame/Core/Interactables/BPI_Gamble.DropBall`
  (`/Game/StealthGame/Core/Interactables/BP_BallSpawner.Drop Ball` (`self.BallSpawner`)))

(event `/Game/StealthGame/Core/Interactables/BPI_Gamble.SwapCam`
  (params (OnPlayer :type Boolean))
  (bind _returnvalue (`GameplayStatics.GetPlayerController` 0))
  (if OnPlayer
    (`PlayerController.SetViewTargetWithBlend` _returnvalue (`self.GambleCam`) 1.0 "VTBlend_Linear" 0.0 false)
    (`KismetSystemLibrary.PrintString` "Swapping to Gamble Cam")
    (else
      (bind _asbp_third_person_character_custom (cast `/Game/StealthGame/Core/Characters/PlayerCharacter/BP_ThirdPersonCharacterCustom` (`GameplayStatics.GetPlayerPawn` 0)))
      (`PlayerController.SetViewTargetWithBlend` _returnvalue _asbp_third_person_character_custom 0.0 "VTBlend_Linear" 0.0 false)
      (`KismetSystemLibrary.PrintString` "Swapping to Normal Cam"))))

(fn `UserConstructionScript`)