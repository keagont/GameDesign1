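; Scoring bin for a gambling ball minigame that multiplies the player's score when a BP_Ball lands in it.
; On BeginPlay it derives its multiplier from a quartic curve of X distance from a hardcoded center, so outer bins pay more, then rounds it up to tenths and displays it.
; Box overlap destroys the ball and passes the multiplier to MultScore on the player character's GambleMenu.
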(event `self.ReceiveBeginPlay`
  (bind _returnvalue_x (`KismetMathLibrary.BreakVector` (`self.K2_GetActorLocation`)))
  (bind _returnvalue (/ (`KismetMathLibrary.Abs` (- _returnvalue_x 1500.0)) 1270.0))
  (bind _returnvalue_2 (+ 0.2 (* 4.8 (* _returnvalue _returnvalue _returnvalue _returnvalue))))
  (bind _returnvalue_3 (`KismetMathLibrary.FFloor` _returnvalue_2))
  (bind _output_get (set `self.ScoreMult` (+ _returnvalue_3 (/ (`KismetMathLibrary.FCeil` (* (- _returnvalue_2 _returnvalue_3) 10.0)) 10))))
  (`TextRenderComponent.K2_SetText` (`self.Score Mult`) (`KismetTextLibrary.Conv_StringToText` (`KismetStringLibrary.Concat_StrStr` (`KismetTextLibrary.Conv_TextToString` (`KismetTextLibrary.Conv_DoubleToText` _output_get "HalfToEven")) "x"))))

(event `self.Box.OnComponentBeginOverlap`
  (params (OverlappedComponent :type "PrimitiveComponent Object Reference") (OtherActor :type "Actor Object Reference") (OtherComp :type "PrimitiveComponent Object Reference") (OtherBodyIndex :type Integer) (bFromSweep :type Boolean) (SweepResult :type "HitResult Structure (by ref)"))
  (bind _asbp_ball (cast `/Game/StealthGame/Core/Interactables/BP_Ball` OtherActor))
  (`self.K2_DestroyActor` _asbp_ball)
  (bind _asbp_third_person_character_custom (cast `/Game/StealthGame/Core/Characters/PlayerCharacter/BP_ThirdPersonCharacterCustom` (`GameplayStatics.GetPlayerCharacter` 0)))
  (`/Game/StealthGame/Core/Characters/PlayerCharacter/Widgets/W_GambleInterface.MultScore` (`/Game/StealthGame/Core/Characters/PlayerCharacter/BP_ThirdPersonCharacterCustom.GambleMenu` _asbp_third_person_character_custom) (`self.ScoreMult`)))

(fn `UserConstructionScript`)